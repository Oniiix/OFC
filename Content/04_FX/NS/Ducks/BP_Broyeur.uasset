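; BP_Broyeur is a grinder prop made of rows of blades that turn in opposite directions.
; The construction script spaces blades along X from NBBlades and SpacingBlades, using a FlipFlop to alternate them between two instanced static mesh components, the second set rotated half a turn.
; On BeginPlay a Timeline drives rotator lerps that spin two scene components a full turn in opposite senses, offset by half a turn.
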(event `self.ReceiveBeginPlay`
  (bind (_direction _newtrack_0) (`Timeline|Timeline` :!via `PlayFromStart`)
    (:`Update`
      (`SceneComponent.K2_SetRelativeRotation` (`self.Scene`) (`KismetMathLibrary.RLerp` (struct) (struct :`Roll` -360.0) _newtrack_0) false false)
      (`SceneComponent.K2_SetRelativeRotation` (`self.Scene1`) (`KismetMathLibrary.RLerp` (struct :`Roll` -180.0) (struct :`Roll` 180.0) _newtrack_0) false false))))

(fn `UserConstructionScript`
  (bind _instancedstaticmesh (`self.InstancedStaticMesh`))
  (bind _instancedstaticmesh1 (`self.InstancedStaticMesh1`))
  (bind _static_mesh (`self.static mesh`))
  (bind _instance_transforms_0 (`self.Instance Transforms_0`))
  (for _index (range (+ (`self.NB Blades`) 1))
    (`/Engine/EditorBlueprintResources/StandardMacros.FlipFlop`
      (:`A`
        (set `self.Rotation` (struct))
        (bind _returnvalue (`KismetMathLibrary.MakeTransform` (`KismetMathLibrary.MakeVector` (* _index (`self.Spacing Blades`))) (`self.Rotation`)))
        (`KismetArrayLibrary.Array_AddUnique` (`self.Instance Transforms`) _returnvalue))
      (:`B`
        (set `self.Rotation` (struct :`Yaw` 180.0))
        (`KismetArrayLibrary.Array_AddUnique` _instance_transforms_0 _returnvalue))))
  (`InstancedStaticMeshComponent.AddInstances` _instancedstaticmesh (`self.Instance Transforms`) false false true)
  (`StaticMeshComponent.SetStaticMesh` _instancedstaticmesh _static_mesh)
  (`InstancedStaticMeshComponent.AddInstances` _instancedstaticmesh1 _instance_transforms_0 false false true)
  (`StaticMeshComponent.SetStaticMesh` _instancedstaticmesh1 _static_mesh))