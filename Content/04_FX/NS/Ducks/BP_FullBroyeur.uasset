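; Grinder ("Broyeur") actor that stages the end-credits duck set piece with trapdoors, Niagara effects and sound.
; BeginPlay starts ambience, swings both trapdoors open by timeline, then runs staggered CoinDeath and Nuggets systems before reversing the doors.
; CoinDeath receives the Blueprint as a Niagara object variable for the ParticleData callback.
; That callback plays scared-duck sounds with timeline-driven pitch, animates an end-screen material collection parameter and queues the credits music once.
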(event `self.ReceiveBeginPlay`
  (bind _coin_death (`self.Coin death`))
  (bind _nuggets (`self.Nuggets`))
  (`|ExecutionSequence`
    (:`then_0`
      ;[1 1 1] Ambience Sounds
      (`/Engine/EditorBlueprintResources/StandardMacros.DoOnce` false
        (:`Completed`
          (`GameplayStatics.PlaySound2D` (`self.Credits Amb Sounds`) 0.68 1.0 0.0 null null false))))
    (:`then_1`
      (`KismetSystemLibrary.Delay` 2.0)
      (bind (_direction _newtrack_0) (`Timeline|Timeline` :!via `PlayFromStart`)
        (:`Update`
          (`|ExecutionSequence`
            (:`then_0`
              (`/Engine/EditorBlueprintResources/StandardMacros.DoOnce` false
                (:`Completed`
                  ;[1 1 1] SFX Trapdoor
                  (`GameplayStatics.PlaySoundAtLocation` (`self.Trapdoor_Open_SFX`) (`SceneComponent.K2_GetComponentLocation` (`self.Trapdoor`)) (struct) (`self.Trapdoor_Open_Volume`) 1.0 0.0 null null null null))))
            (:`then_1`
              (`SceneComponent.K2_SetRelativeRotation` (`self.Trap_door`) (`KismetMathLibrary.RLerp` (struct :`Yaw` 180.0) (struct :`Yaw` 180.0 :`Roll` -90.0) _newtrack_0) false false)
              (`SceneComponent.K2_SetRelativeRotation` (`self.Trap_door1`) (`KismetMathLibrary.RLerp` (struct) (struct :`Roll` -90.0) _newtrack_0) false false))))
        (:`Finished`
          (`ActorComponent.SetActive` _coin_death true false)
          (`NiagaraComponent.SetNiagaraVariableObject` _coin_death "BP" self)
          (`NiagaraComponent.SetVariableFloat` _coin_death "Offset Spawn" (`self.Spawnoffset`))
          (`NiagaraComponent.SetVariableFloat` _nuggets "Death Zone Z offset" (`self.Nuggets death zone`))
          (`KismetSystemLibrary.Delay` 3.0)
          (`ActorComponent.SetActive` _nuggets true false)
          (`KismetSystemLibrary.Delay` 10.0)
          (`ActorComponent.SetActive` (`self.Coin death`) false false)
          (`KismetSystemLibrary.Delay` 2.0)
          (`ActorComponent.SetActive` (`self.Nuggets`) false false)
          (bind (_direction_2 _newtrack_0_2) (`Timeline|Timeline_0` :!via `ReverseFromEnd`)
            (:`Update`
              (`SceneComponent.K2_SetRelativeRotation` (`self.Trap_door`) (`KismetMathLibrary.RLerp` (struct :`Yaw` 180.0) (struct :`Yaw` 180.0 :`Roll` -90.0) _newtrack_0_2) false false)
              (`SceneComponent.K2_SetRelativeRotation` (`self.Trap_door1`) (`KismetMathLibrary.RLerp` (struct) (struct :`Roll` -90.0)) false false))))))))

(event `self.ReceiveParticleData`
  (params (Data :type "Array of BasicParticleData Structure (by ref)") (NiagaraSystem :type "NiagaraSystem Object Reference") (SimulationPositionOffset :type "Vector Structure (by ref)"))
  (`|ExecutionSequence`
    (:`then_0`
      (`GameplayStatics.PlaySound2D` "/Game/05_Audio/SFX/Metasounds/Duck/Duck_Scared/MSS_Duck_Scared.MSS_Duck_Scared" 0.13 (`self.SoundPitch`) 0.0 null null)
      (bind (_direction _pitch _newtrack_1) (`Timeline|PitchDown`)
        (:`Update`
          _)
        (:`Finished`
          _))
      (set `self.SoundPitch` _pitch)
      (`KismetMaterialLibrary.SetScalarParameterValue` "/Game/04_FX/Ressources/PP.PP" "End Sreen" _newtrack_1))
    (:`then_1`
      ;[1 1 1] End Credit Music
      (`/Engine/EditorBlueprintResources/StandardMacros.DoOnce` false
        (:`Completed`
          (`KismetSystemLibrary.Delay` 13.8)
          (`GameplayStatics.PlaySound2D` "/Game/05_Audio/Music/Credits_Music/MSS_Credits_Music_v2.MSS_Credits_Music_v2" 0.4 1.0 0.0 null null false))))))

(fn `UserConstructionScript`
  (`SceneComponent.K2_SetRelativeLocation` (`self.Trapdoor`) (`KismetMathLibrary.MakeVector` 0.0 0.0 (`self.Trapdoor_height`)) false false))