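; Game mode that runs the wave loop, point economy and upgrades of a duck and bubble game.
; It constructs an AI manager at BeginPlay; each wave end scores ducks overlapping the enclosure's count box and explodes all bubbles, and the last wave opens the credits level.
; Upgrade functions spend points and raise levels in a struct map.
; Tick prints duck-count debug text, and bubble switcher setup is left unwired.
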(event `self.ReceiveBeginPlay`
  (`|ExecutionSequence`
    (:`then_0`
      (bind _outactors (`GameplayStatics.GetAllActorsOfClass` "/Game/00_Prog/Game/GPE/BP_EnclosureActor.BP_EnclosureActor_C"))
      (set `self.Enclos` (`|GetArrayItem` _outactors)))
    (:`then_1`
      (bind _returnvalue (`|GenericCreateObject` (`self.AIManagerRef`)))
      (bind _output_get (set `self.AIManager` _returnvalue))
      (`AIManager.Init` _output_get self)
      (add `AIManager.onFinishAllWawes` _output_get (delegate `onFinishAllWawes_Event`))
      (add `AIManager.onEndWave` _output_get (delegate `onEndWave_Event`)))))

(event `onFinishAllWawes_Event`
  (`GameplayStatics.OpenLevelBySoftObjectPtr` "/Game/02_LD/P_Credits.P_Credits"))

(event `onEndWave_Event`
  (`self.Add Point` (`KismetArrayLibrary.Array_Length` (`PrimitiveComponent.GetOverlappingActors` (`/Game/00_Prog/Game/GPE/BP_EnclosureActor.FinalCountBox` (`self.Enclos`)) "/Game/00_Prog/IA/BP_Duck.BP_Duck_C")))
  (`|ExecutionSequence`
    (:`then_0`
      (bind _outactors (`GameplayStatics.GetAllActorsOfClass` "/Game/00_Prog/Game/GPE/Bubble/BP_Bubble.BP_Bubble_C"))
      (bind (_arrayindex _arrayelement) (`/Engine/EditorBlueprintResources/StandardMacros.ReverseForEachLoop` _outactors)
        (:`LoopBody`
          (`/Game/00_Prog/Game/GPE/Bubble/BP_Bubble.Explode` _arrayelement))))))

(event `self.ReceiveTick`
  (params (DeltaSeconds :type "Float (single-precision)"))
  (`KismetSystemLibrary.PrintString` (`KismetStringLibrary.Concat_StrStr` (`KismetStringLibrary.Conv_IntToString` (`AIManager.GetFreeDuck` (`self.AIManager`))) "in Free duck") true true (struct :`G` 0.023676 :`B` 1.0 :`A` 1.0) DeltaSeconds)
  (`KismetSystemLibrary.PrintString` (`KismetStringLibrary.Concat_StrStr` (`KismetStringLibrary.Conv_IntToString` (`AIManager.GetDuckCount` (`self.AIManager`))) "in duck list") true true (struct :`G` 0.023676 :`B` 1.0 :`A` 1.0) DeltaSeconds))

(fn `Add Point`
  (params (`Point To add` :type Integer))
  (bind _output_get (set `self.Point` (+ (`self.Point`) `Point To add`)))
  (`KismetSystemLibrary.PrintString` (`KismetStringLibrary.Conv_IntToString` _output_get)))

(fn `Has Point`
  (params (`Point Needed` :type Integer))
  (returns (`Has Point` :type Boolean))
  (return (>= (`self.Point`) `Point Needed`)))

(fn `Remove Point`
  (params (`Point to remove` :type Integer))
  (set `self.Point` (- (`self.Point`) `Point to remove`))
  (`KismetSystemLibrary.PrintString` "Hello"))

(fn `UnlockSwitchersByType`
  (params (bubbleSwitchType :type "/Game/00_Prog/Game/GPE/Bubble/BP_Bubble Class Reference"))
  (bind _bubbleswitchers (`self.bubbleSwitchers`))
  (if (`KismetArrayLibrary.Array_IsNotEmpty` _bubbleswitchers)
    (for _array_element _bubbleswitchers
      (if (== bubbleSwitchType (`/Game/00_Prog/Game/GPE/Bubble/Switcher/BP_BubbleSwitcher.bubbleSwitchType` _array_element))
        (if (`/Game/00_Prog/Game/GPE/Bubble/Switcher/BP_BubbleSwitcher.isUnlocked` _array_element)
          (`/Game/00_Prog/Game/GPE/Bubble/Switcher/BP_BubbleSwitcher.UnlockSwitcher` _array_element))))))

(fn `Upgrade Level Fire Rate`
  (locals (Enum :type "UEnumUpgradeType Enum"))
  (bind _value (`BlueprintMapLibrary.Map_Find` (`self.Upgrades`) (`local.Enum`)))
  (bind (_name _level _prices) (break `/Game/00_Prog/UI/Bp_UpgradeStruct` _value))
  (`self.Remove Point` (`|GetArrayItem` _prices _level))
  (bind _structout (setmembers `/Game/00_Prog/UI/Bp_UpgradeStruct` :`StructRef` _value :`Level` (+ _level 1)))
  (`BlueprintMapLibrary.Map_Add` (`self.Upgrades`) (`local.Enum`) _structout))

(fn `Upgrade Shooting Power`
  (locals (Enum :type "UEnumUpgradeType Enum" :default "ShootingPower"))
  (bind _value (`BlueprintMapLibrary.Map_Find` (`self.Upgrades`) (`local.Enum`)))
  (bind (_name _level _prices) (break `/Game/00_Prog/UI/Bp_UpgradeStruct` _value))
  (`self.Remove Point` (`|GetArrayItem` _prices _level))
  (bind _structout (setmembers `/Game/00_Prog/UI/Bp_UpgradeStruct` :`StructRef` _value :`Level` (+ _level 1)))
  (`BlueprintMapLibrary.Map_Add` (`self.Upgrades`) (`local.Enum`) _structout))

(fn `Upgrade Suction Speed `
  (locals (enum :type "UEnumUpgradeType Enum" :default "SuctionSpeed"))
  (bind _value (`BlueprintMapLibrary.Map_Find` (`self.Upgrades`) (`local.Enum`)))
  (bind (_name _level _prices) (break `/Game/00_Prog/UI/Bp_UpgradeStruct` _value))
  (`self.Remove Point` (`|GetArrayItem` _prices _level))
  (bind _structout (setmembers `/Game/00_Prog/UI/Bp_UpgradeStruct` :`StructRef` _value :`Level` (+ _level 1)))
  (`BlueprintMapLibrary.Map_Add` (`self.Upgrades`) (`local.Enum`) _structout))

(fn `UserConstructionScript`)