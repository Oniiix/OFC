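; BP_BubbleSwitch is a floating bubble tied to a Switcher actor and carrying a bubble type (soap, chewing gum, oil, mercury).
; On BeginPlay it stores its location as target, zeroes projectile gravity, caps speed, unbinds sphere overlaps, then sets Niagara material by type and scale by sphere radius.
; Tick applies drag, and TellSwitcherToRespawnBubble passes the bubble to its Switcher's ChangeBubbleSwitch.
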(event `self.ReceiveBeginPlay`
  (bind _projectilemovement (`self.ProjectileMovement`))
  (set `self.targetLocation` (`self.K2_GetActorLocation`))
  (set `ProjectileMovementComponent.ProjectileGravityScale` 0.0 _projectilemovement)
  (set `ProjectileMovementComponent.MaxSpeed` (`self.CatchMaxSpeed`) _projectilemovement)
  (set `self.canInit` true)
  (clear `PrimitiveComponent.OnComponentBeginOverlap` (`self.Sphere`))
  (`KismetSystemLibrary.DelayUntilNextTick`)
  (`NiagaraComponent.SetVariableMaterial` (`self.Niagara`) "Bubble_Material" (select `/Game/00_Prog/Utils/E_BubbleTypes` (`/Game/00_Prog/Utils/BFL_Bubbles.getBubbleEnumFromClass` (`self.bubbleSwitchType`)) :`NewEnumerator0` "/Game/04_FX/Ressources/Mat/MIFX_Bubble.MIFX_Bubble" :`NewEnumerator1` "/Game/04_FX/Ressources/Mat/MIFX_ChewingGum_Bubble.MIFX_ChewingGum_Bubble" :`NewEnumerator2` "/Game/04_FX/Ressources/Mat/MIFX_Oil_Bubble.MIFX_Oil_Bubble" :`NewEnumerator3` "/Game/04_FX/Ressources/Mat/MIFX_mercury_Bubble.MIFX_mercury_Bubble" :`NewEnumerator4` "/Game/04_FX/Ressources/Mat/MIFX_Nuggets.MIFX_Nuggets" :!type "MaterialInterface Object Reference"))
  (`NiagaraComponent.SetVariableFloat` (`self.Niagara`) "Scale" (`SphereComponent.GetScaledSphereRadius` (`self.Sphere`))))

(event `self.ReceiveTick`
  (params (DeltaSeconds :type "Float (single-precision)"))
  (`self.CalculateDrag` DeltaSeconds))

(fn `TellSwitcherToRespawnBubble`
  (bind _switcher (`self.switcher`))
  (`/Engine/EditorBlueprintResources/StandardMacros.IsValid` _switcher
    (:`Is Valid`
      (`/Game/00_Prog/Game/GPE/Bubble/Switcher/BP_BubbleSwitcher.Change Bubble Switch` _switcher self))))

(fn `UserConstructionScript`
  (`parent.UserConstructionScript`))