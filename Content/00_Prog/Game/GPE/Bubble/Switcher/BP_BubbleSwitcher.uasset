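; BP_BubbleSwitcher is a bubble gameplay element that, once unlocked, shows its flower and supplies two switch bubbles.
; On BeginPlay it registers with BP_OFCGameModeBase's switcher list and unlocks itself if already flagged as unlocked.
; Unlocking spawns a bubble at each spawn component, passing it the switch type and a back-reference to the switcher.
; ChangeBubbleSwitch spawns a replacement at the matching slot for a given bubble, without destroying the old one.
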(event `self.ReceiveBeginPlay`
  (bind _asbp_ofcgame_mode_base (cast `/Game/00_Prog/BP_OFCGameModeBase` (`GameplayStatics.GetGameMode`)))
  (`KismetArrayLibrary.Array_Add` (`/Game/00_Prog/BP_OFCGameModeBase.bubbleSwitchers` _asbp_ofcgame_mode_base) self)
  (if (`self.isUnlocked`)
    (`self.UnlockSwitcher`)))

(fn `Change Bubble Switch`
  (params (bubbleToChange :type "/Game/00_Prog/Game/GPE/Bubble/Switcher/BP_BubbleSwitch Object Reference"))
  (if (== bubbleToChange (`self.firstBubble`))
    (bind _newbubbleswitch (`self.SpawnBubbleSwitch` (`self.FirstBubbleSpawn`)))
    (set `self.firstBubble` _newbubbleswitch)
    (elif (== bubbleToChange (`self.secondBubble`))
      (bind _newbubbleswitch_2 (`self.SpawnBubbleSwitch` (`self.SecondBubbleSpawn`)))
      (set `self.secondBubble` _newbubbleswitch_2))))

(fn `SetupBubbles`
  (bind _newbubbleswitch (`self.SpawnBubbleSwitch` (`self.FirstBubbleSpawn`)))
  (set `self.firstBubble` _newbubbleswitch)
  (bind _newbubbleswitch_2 (`self.SpawnBubbleSwitch` (`self.SecondBubbleSpawn`)))
  (set `self.secondBubble` _newbubbleswitch_2))

(fn `SpawnBubbleSwitch`
  (params (spawnComponent :type "SceneComponent Object Reference"))
  (returns (newBubbleSwitch :type "/Game/00_Prog/Game/GPE/Bubble/Switcher/BP_BubbleSwitch Object Reference"))
  (bind _returnvalue (`|SpawnActorFromClass` (`self.spawnedBubble`) (`SceneComponent.K2_GetComponentToWorld` spawnComponent) "Undefined" "MultiplyWithRoot" null null))
  (set `/Game/00_Prog/Game/GPE/Bubble/Switcher/BP_BubbleSwitch.bubbleSwitchType` (`self.bubbleSwitchType`) _returnvalue)
  (set `/Game/00_Prog/Game/GPE/Bubble/Switcher/BP_BubbleSwitch.switcher` self _returnvalue)
  (return _returnvalue))

(fn `UnlockSwitcher`
  (bind _flower (`self.Flower`))
  (`self.SetupBubbles`)
  (`SceneComponent.SetVisibility` _flower true false)
  (`SceneComponent.SetHiddenInGame` _flower false false)
  (`PrimitiveComponent.SetCollisionEnabled` _flower "NoCollision")
  (set `PrimitiveComponent.bGenerateOverlapEvents` true _flower)
  (set `PrimitiveComponent.CanCharacterStepUpOn` "ECB_Yes" _flower)
  (set `self.isUnlocked` true))

(fn `UserConstructionScript`)