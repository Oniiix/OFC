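; Bubble projectile that captures actors with a CaughtComponent and can then be sucked in, held by the weapon and thrown.
; A catch enlarges the bubble, adds drag and starts an auto-pop timer; holding pauses collision and the timer.
; Once nearly stopped, it lerps to a hover point found by a downward ground trace.
; Hits pop it, releasing the captive, while piercing-tagged hits explode it, destroying both.
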(event `self.ReceiveBeginPlay`
  (bind _niagara (`self.Niagara`))
  (`|ExecutionSequence`
    (:`then_0`
      (set `ProjectileMovementComponent.MaxSpeed` (`self.ShootMaxSpeed`) (`self.ProjectileMovement`))
      (`NiagaraComponent.SetVariableMaterial` _niagara "Bubble_Material" (`self.NiagaraMat`))
      (`NiagaraComponent.SetVariableFloat` _niagara "Scale" (`SphereComponent.GetScaledSphereRadius` (`self.Sphere`)))
      (set `self.ThrowGravity` (`ProjectileMovementComponent.ProjectileGravityScale` (`self.ProjectileMovement`))))))

(event `self.ReceiveTick`
  (params (DeltaSeconds :type "Float (single-precision)"))
  (bind (_returnvalue_x _returnvalue_y) (`KismetMathLibrary.BreakVector` (`self.K2_GetActorLocation`)))
  (bind (_targetlocation_x _targetlocation_y) (`KismetMathLibrary.BreakVector` (`self.targetLocation`)))
  (`|ExecutionSequence`
    (:`then_0`
      (bind _output_get (set `self.canInit` (and (== (`MovementComponent.Velocity` (`self.ProjectileMovement`)) (0.0 0.0 0.0) :`ErrorTolerance` 4.0) (not (`self.isHold`)))))
      (if (and _output_get (!= (`KismetMathLibrary.MakeVector` _targetlocation_x _targetlocation_y) (`KismetMathLibrary.MakeVector` _returnvalue_x _returnvalue_y) :`ErrorTolerance` 10.0))
        (`self.ComputeTragetLocation`)))
    (:`then_1`
      (if (`self.canInit`)
        (`self.K2_SetActorLocation` (`KismetMathLibrary.VLerp` (`self.K2_GetActorLocation`) (`self.targetLocation`) (* DeltaSeconds (`self.InitSpeed`))))))
    (:`then_2`
      (`self.CalculateDrag` DeltaSeconds)
      (set `self.lastLocation` (`self.K2_GetActorLocation`)))))

(event `self.Sphere.OnComponentHit`
  (params (HitComponent :type "PrimitiveComponent Object Reference") (OtherActor :type "Actor Object Reference") (OtherComp :type "PrimitiveComponent Object Reference") (NormalImpulse :type "Vector Structure") (Hit :type "HitResult Structure (by ref)"))
  ;[1 1 1] Pop Bubble
  (`self.Touch` OtherActor OtherComp))

(event `self.Sphere.OnComponentBeginOverlap`
  (params (OverlappedComponent :type "PrimitiveComponent Object Reference") (OtherActor :type "Actor Object Reference") (OtherComp :type "PrimitiveComponent Object Reference") (OtherBodyIndex :type Integer) (bFromSweep :type Boolean) (SweepResult :type "HitResult Structure (by ref)"))
  ;[1 1 1] Catch Actor
  (bind _successcatch (`self.Catch` OtherActor))
  (if _successcatch
    (`self.ComputeTragetLocation`)))

(event `self.ProjectileMovement.OnProjectileStop`
  (params (ImpactResult :type "HitResult Structure (by ref)")))

(event `/Game/00_Prog/Utils/BI_Bubble.OnHeld`
  (bind _capturedactor (`self.capturedActor`)
    (:`then`
      (message `/Game/00_Prog/Utils/BI_Bubble.OnHeld` _capturedactor))
    (:`else`)))

(event `self.PopBubble`
  (`self.Pop`))

(fn `CalculateDrag`
  (params (Delta :type "Float (double-precision)"))
  (if (`self.Drag?`)
    (set `MovementComponent.Velocity` (- (`MovementComponent.Velocity` (`self.ProjectileMovement`)) (* (`KismetMathLibrary.Normal` (`MovementComponent.Velocity` (`self.ProjectileMovement`))) (`self.DragForce`) Delta)) (`self.ProjectileMovement`))))

(fn `Catch`
  (params (catchActor :type "Actor Object Reference"))
  (returns (successCatch :type Boolean))
  (bind _returnvalue (`self.GetComponentByClass` catchActor "/Script/OFC.CaughtComponent"))
  (if (`KismetSystemLibrary.IsValid` (`self.capturedActor`))
    (return false)
    (elif (`KismetSystemLibrary.IsValid` _returnvalue)
      (if (`CaughtComponent.IsInBubble` _returnvalue)
        (return false)
        (else
          (bind _output_get (set `self.capturedActor` catchActor))
          (`KismetSystemLibrary.PrintString` "Hello")
          (`CaughtComponent.onCaught` _returnvalue self)
          (`self.SetActorInBubble` _output_get)
          (`SphereComponent.SetSphereRadius` (`self.Sphere`) 50.0 true)
          (`self.StartTimer`)
          (set `ProjectileMovementComponent.MaxSpeed` (`self.CatchMaxSpeed`) (`self.ProjectileMovement`))
          (set `self.Drag?` true)
          (set `self.NewBubble?` false)
          (`GameplayStatics.PlaySoundAtLocation` "/Game/05_Audio/SFX/Metasounds/Bubbles/Bubble_Type5/MSS_Bubble_Type5.MSS_Bubble_Type5" (`self.K2_GetActorLocation`) (struct) 0.5 1.0 0.1 null null null null)
          (return true)))
      (else
        (return false)))))

(fn `CaughtByWeapon`
  (bind _projectilemovement (`self.ProjectileMovement`))
  (set `MovementComponent.Velocity` (0.0 0.0 0.0) _projectilemovement)
  (set `ProjectileMovementComponent.ProjectileGravityScale` 0.0 _projectilemovement)
  (`KismetSystemLibrary.K2_ClearAndInvalidateTimerHandle` (`self.PopTimer`))
  (`PrimitiveComponent.SetCollisionEnabled` (`self.Sphere`) "NoCollision")
  (set `self.isHold` true)
  (set `self.canInit` false)
  (`self.onStartHold`))

(fn `ComputeTragetLocation`
  (bind _returnvalue (`self.K2_GetActorLocation`))
  (bind _outhit (`KismetSystemLibrary.SphereTraceSingleForObjects` _returnvalue (- _returnvalue (0.0 0.0 1000.0)) (`SphereComponent.SphereRadius` (`self.Sphere`)) (`self.groundLayer`)))
  (`KismetSystemLibrary.DrawDebugSphere` (`.Location` (`GameplayStatics.BreakHitResult` _outhit)) 100.0 12 (struct :`R` 1.0 :`G` 1.0 :`B` 1.0 :`A` 1.0) 5.0)
  (set `self.targetLocation` (+ (`.Location` (`GameplayStatics.BreakHitResult` _outhit)) (`KismetMathLibrary.MakeVector` 0.0 0.0 (`self.groundOffset`))))
  (set `MovementComponent.Velocity` (0.0 0.0 0.0) (`self.ProjectileMovement`))
  (set `ProjectileMovementComponent.ProjectileGravityScale` 0.0 (`self.ProjectileMovement`)))

(fn `Explode`
  (`GameplayStatics.PlaySoundAtLocation` (`self.SFX_Explode_2`) (`self.K2_GetActorLocation`) (struct) 0.22 1.0 0.0 null null null null)
  (bind _capturedactor (`self.capturedActor`)
    (:`then`
      (`|ExecutionSequence`
        (:`then_0`
          (bind _asbp_duck (cast `/Game/00_Prog/IA/BP_Duck` _capturedactor))
          (`GameplayStatics.PlaySoundAtLocation` "/Game/05_Audio/SFX/Metasounds/Bubbles/Bubble_Burst/MSS_Bubble_Burst_Light.MSS_Bubble_Burst_Light" (`self.K2_GetActorLocation` _asbp_duck) (struct) 0.75 1.0 0.0 null null null null))
        (:`then_1`
          (`CaughtComponent.onExplode` (`self.GetComponentByClass` _capturedactor "/Script/OFC.CaughtComponent"))
          (bind _returnvalue (`NiagaraFunctionLibrary.SpawnSystemAtLocation` "/Game/04_FX/NS/Player/NS_BubblePop.NS_BubblePop" (`self.K2_GetActorLocation`) (`KismetMathLibrary.MakeRotFromX` (- (0.0 0.0 0.0) (`MovementComponent.Velocity` (`self.ProjectileMovement`))))))
          (`NiagaraComponent.SetVariableMaterial` _returnvalue "Bubble_Mat" (`self.NiagaraMat`))
          (`self.SetLifeSpan` (`self.capturedActor`) 0.05)
          (`self.SetLifeSpan` 0.05))))
    (:`else`)))

(fn `Pop`
  (`GameplayStatics.PlaySoundAtLocation` (`self.SFX_Pop`) (`self.K2_GetActorLocation`) (struct) 0.75 1.0 0.0 null null null null)
  (bind _returnvalue (`NiagaraFunctionLibrary.SpawnSystemAtLocation` "/Game/04_FX/NS/Player/NS_BubblePop.NS_BubblePop" (`self.K2_GetActorLocation`) (`KismetMathLibrary.MakeRotFromX` (`KismetMathLibrary.MakeVector` 0.0 0.0 1.0))))
  (`NiagaraComponent.SetVariableMaterial` _returnvalue "Bubble_Mat" (`self.NiagaraMat`))
  (`self.K2_DestroyActor`)
  (bind _capturedactor (`self.capturedActor`)
    (:`then`
      (`CaughtComponent.onPop` (`self.GetComponentByClass` _capturedactor "/Script/OFC.CaughtComponent")))
    (:`else`)))

(fn `Shoot`
  (params (ShootDirection :type "Vector Structure"))
  (set `MovementComponent.Velocity` ShootDirection (`self.ProjectileMovement`))
  (set `ProjectileMovementComponent.MaxSpeed` (`self.ShootMaxSpeed`) (`self.ProjectileMovement`))
  (set `self.Drag?` false)
  (`GameplayStatics.PlaySound2D` (`self.SFX_Shoot`) 1.0 1.0 0.0 null null))

(fn `StartTimer`
  (if (`KismetSystemLibrary.K2_IsValidTimerHandle` (`self.PopTimer`))
    (`KismetSystemLibrary.K2_ClearAndInvalidateTimerHandle` (`self.PopTimer`)))
  (bind _returnvalue (`KismetSystemLibrary.K2_SetTimer` null "Pop" (`self.autoPopTimer`)))
  (set `self.PopTimer` _returnvalue))

(fn `Suck`
  (params (suckForce :type "Vector Structure") (RotationSpeed :type "Float (double-precision)"))
  (bind _returnvalue (`KismetMathLibrary.VSize` (`MovementComponent.Velocity` (`self.ProjectileMovement`))))
  (if (not (`self.NewBubble?`))
    (set `MovementComponent.Velocity` (+ (* suckForce (`GameplayStatics.GetWorldDeltaSeconds`) (`self.SuckSpeedMod`)) (`MovementComponent.Velocity` (`self.ProjectileMovement`))) (`self.ProjectileMovement`))
    (set `MovementComponent.Velocity` (* (`KismetMathLibrary.GetForwardVector` (`KismetMathLibrary.RInterpTo` (`KismetMathLibrary.MakeRotFromX` (`MovementComponent.Velocity` (`self.ProjectileMovement`))) (`KismetMathLibrary.MakeRotFromX` suckForce) (`GameplayStatics.GetWorldDeltaSeconds`) RotationSpeed)) (- _returnvalue (* _returnvalue (`self.SuckRotDragPercent`) (`GameplayStatics.GetWorldDeltaSeconds`)))) (`self.ProjectileMovement`))))

(fn `Throw`
  (params (ThrowDirection :type "Vector Structure"))
  (bind _projectilemovement (`self.ProjectileMovement`))
  (set `MovementComponent.Velocity` ThrowDirection _projectilemovement)
  (set `ProjectileMovementComponent.ProjectileGravityScale` (`self.ThrowGravity`) _projectilemovement)
  (set `ProjectileMovementComponent.MaxSpeed` (`self.ShootMaxSpeed`) _projectilemovement)
  (set `self.Drag?` false)
  (`PrimitiveComponent.SetCollisionEnabled` (`self.Sphere`) "QueryAndPhysics")
  (`GameplayStatics.PlaySound2D` (`self.SFX_Shoot`) 1.0 1.0 0.0 null null)
  (bind _returnvalue (`NiagaraFunctionLibrary.SpawnSystemAtLocation` "/Game/04_FX/NS/Player/NS_Gun_Shoot.NS_Gun_Shoot" (`self.K2_GetActorLocation`) (`KismetMathLibrary.MakeRotFromX` (`KismetMathLibrary.MakeVector` 0.0 0.0 1.0))))
  (`NiagaraComponent.SetVariableMaterial` _returnvalue "Bubble_Mat" (`self.NiagaraMat`))
  (`self.StartTimer`)
  (set `self.isHold` false)
  (bind _capturedactor (`self.capturedActor`)
    (:`then`
      (message `/Game/00_Prog/Utils/BI_Bubble.OnThrown` _capturedactor)
      (`self.onThrow`))
    (:`else`)))

(fn `Touch`
  (params (TouchActor :type "Actor Object Reference") (TouchComponent :type "ActorComponent Object Reference"))
  (if (`ActorComponent.ComponentHasTag` TouchComponent (`/Game/00_Prog/Utils/BFL_Piercing.GetPiercingTagName`))
    (`self.Explode` :!label _label)
    (elif (`self.ActorHasTag` TouchActor (`/Game/00_Prog/Utils/BFL_Piercing.GetPiercingTagName`))
      (goto _label)
      (else
        (`self.Pop`)))))

(fn `UserConstructionScript`)