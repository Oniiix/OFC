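; BP_MercuryBubble is a bubble gameplay element with a timed auto-pop.
; StartTimer clears any valid PopTimer, then schedules the Explode function by name after AutoPopTimer, so each call restarts the countdown.
; The event graph holds only disabled default events and the construction script just calls its parent; Explode is not defined in these graphs.
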(fn `StartTimer`
  (if (`KismetSystemLibrary.K2_IsValidTimerHandle` (`self.PopTimer`))
    (`KismetSystemLibrary.K2_ClearAndInvalidateTimerHandle` (`self.PopTimer`)))
  (bind _returnvalue (`KismetSystemLibrary.K2_SetTimer` null "Explode" (`self.autoPopTimer`)))
  (set `self.PopTimer` _returnvalue))

(fn `UserConstructionScript`
  (`parent.UserConstructionScript`))