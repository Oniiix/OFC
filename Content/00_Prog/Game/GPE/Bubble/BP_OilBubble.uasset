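; Oil bubble Blueprint: a projectile that can capture one actor and explodes when touched by a piercing-tagged component or actor.
; BeginPlay starts a timer, and each bounce spawns a Niagara effect using the oil bubble material.
; Catch requires an empty bubble and an uncaught actor with a CaughtComponent, then notifies it and resizes the sphere.
; Catch's velocity adjustment and true return are disconnected, and ComputeTragetLocation is empty.
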(event `self.ReceiveBeginPlay`
  (`parent.ReceiveBeginPlay`)
  (`self.StartTimer`))

(event `self.ReceiveTick`
  (params (DeltaSeconds :type "Float (single-precision)")))

(event `self.ProjectileMovement.OnProjectileBounce`
  (params (ImpactResult :type "HitResult Structure (by ref)") (ImpactVelocity :type "Vector Structure (by ref)"))
  (bind (_bblockinghit _binitialoverlap _time _distance _location _impactpoint _normal) (`GameplayStatics.BreakHitResult` ImpactResult))
  (bind _returnvalue (`NiagaraFunctionLibrary.SpawnSystemAtLocation` "/Game/04_FX/NS/Player/NS_Bubble_bounce.NS_Bubble_bounce" _impactpoint (`KismetMathLibrary.MakeRotFromX` _normal)))
  (`NiagaraComponent.SetVariableMaterial` _returnvalue "Bubble_Mat" "/Game/04_FX/Ressources/Mat/MIFX_Oil_Bubble.MIFX_Oil_Bubble"))

(fn `Catch`
  (params (catchActor :type "Actor Object Reference"))
  (returns (successCatch :type Boolean))
  (bind _returnvalue (`self.GetComponentByClass` catchActor "/Script/OFC.CaughtComponent"))
  (if (`KismetSystemLibrary.IsValid` (`self.capturedActor`))
    (return false)
    (elif (`KismetSystemLibrary.IsValid` _returnvalue)
      (if (`CaughtComponent.IsInBubble` _returnvalue)
        (return false)
        (else
          (set `self.capturedActor` catchActor)
          (`CaughtComponent.onCaught` _returnvalue self)
          (`SphereComponent.SetSphereRadius` (`self.Sphere`) 50.0 true)
          (set `self.NewBubble?` false)))
      (else
        (return false)))))

(fn `ComputeTragetLocation`)

(fn `Touch`
  (params (TouchActor :type "Actor Object Reference") (TouchComponent :type "ActorComponent Object Reference"))
  (if (`ActorComponent.ComponentHasTag` TouchComponent (`/Game/00_Prog/Utils/BFL_Piercing.GetPiercingTagName`))
    (`self.Explode` :!label _label)
    (elif (`self.ActorHasTag` TouchActor (`/Game/00_Prog/Utils/BFL_Piercing.GetPiercingTagName`))
      (goto _label))))

(fn `UserConstructionScript`
  (`parent.UserConstructionScript`))