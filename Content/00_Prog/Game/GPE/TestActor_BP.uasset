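; TestActor_BP is a test gameplay element that can be caught by a bubble.
; On BeginPlay it initializes its Caught component and binds to that component's caught and pop events.
; When caught, it snaps onto the Bubble actor and disables its static mesh collision.
; On pop, it detaches in place and restores query and physics collision.
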(event `self.ReceiveBeginPlay`
  (bind _caught (`self.Caught`))
  (`CaughtComponent.InitCaught` _caught)
  (add `CaughtComponent.onCaught` _caught (delegate `onCaught_Event`))
  (add `CaughtComponent.onPop` (`self.Caught`) (delegate `onPop_Event`)))

(event `onPop_Event`
  (`self.K2_DetachFromActor` "KeepWorld" "KeepWorld" "KeepWorld")
  (`PrimitiveComponent.SetCollisionEnabled` (`self.StaticMesh`) "QueryAndPhysics"))

(event `onCaught_Event`
  (params (_bubble :type "BubbleActor Object Reference"))
  (`self.K2_AttachToActor` _bubble "None" "SnapToTarget" "KeepWorld" "KeepWorld")
  (`PrimitiveComponent.SetCollisionEnabled` (`self.StaticMesh`) "NoCollision"))

(fn `UserConstructionScript`)