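; Duck enclosure actor that tracks captured ducks in an array and with an "InEnclosure" tag.
; Overlap handlers add or remove ducks carried in bubbles or held by the player, while three force fields also remove exiting ducks.
; It registers with the AI manager, supplies Swiper spawn points, surrenders its first duck on attack and empties the array at wave end.
; Its score dispatcher feeds GameMode.AddPoint, but every call to it is disconnected.
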(event `CustomEvent`
  (params (OverlappedComponent :type "PrimitiveComponent Object Reference") (OtherActor :type "Actor Object Reference") (OtherComp :type "PrimitiveComponent Object Reference") (OtherBodyIndex :type Integer) (bFromSweep :type Boolean) (SweepResult :type "HitResult Structure (by ref)")))

(event `OnChangeInDucksArray_Event` :!signature `self.OnChangeInDucksArray`
  (params (ducksNum :type Integer))
  (`/Game/00_Prog/BP_OFCGameModeBase.Add Point` (`self.GameMode`) ducksNum))

(event `onEndWave_Event`
  (`KismetArrayLibrary.Array_Clear` (`self.ducksInEnclosure`)))

(event `self.ReceiveBeginPlay`
  (`KismetSystemLibrary.Delay` 0.2)
  (bind _asbp_ofcgame_mode_base (cast `/Game/00_Prog/BP_OFCGameModeBase` (`GameplayStatics.GetGameMode`))
    (:`then`
      (bind _output_get (set `self.GameMode` _asbp_ofcgame_mode_base))
      (add `self.OnChangeInDucksArray` (delegate `OnChangeInDucksArray_Event`))
      (bind _aimanager (`/Game/00_Prog/BP_OFCGameModeBase.AIManager` _output_get))
      (`AIManager.SetEnclosure` _aimanager self)
      (add `AIManager.onEndWave` _aimanager (delegate `onEndWave_Event`)))
    (:`CastFailed`
      _))
  (add `self.OnActorEndOverlap` (delegate `OnActorEndOverlap_Event`))
  (add `self.OnActorEndOverlap` (delegate `CustomEvent_1`)))

(event `OnActorEndOverlap_Event` :!signature `self.OnActorEndOverlap`
  (params (OverlappedActor :type "Actor Object Reference") (OtherActor :type "Actor Object Reference"))
  (bind _asbp_bubble (cast `/Game/00_Prog/Game/GPE/Bubble/BP_Bubble` OtherActor)
    (:`then`
      (bind _duck (`self.AddDuckFromBubble` _asbp_bubble))
      (if (`KismetSystemLibrary.IsValid` _duck)
        (`KismetSystemLibrary.PrintString` "add point")))
    (:`CastFailed`
      (bind _asbp_main_character (cast `/Game/00_Prog/CCC/BP_MainCharacter` OtherActor))
      (bind _duck_2 (`self.AddDuckFromPlayer` _asbp_main_character))
      (if (`KismetSystemLibrary.IsValid` _duck_2)
        _))))

(event `CustomEvent_1` :!signature `self.OnActorEndOverlap`
  (params (OverlappedActor :type "Actor Object Reference") (OtherActor :type "Actor Object Reference"))
  (bind _enclosurebox (`self.EnclosureBox`))
  (bind _asbp_bubble (cast `/Game/00_Prog/Game/GPE/Bubble/BP_Bubble` OtherActor)
    (:`then`
      (`/Engine/EditorBlueprintResources/StandardMacros.IsValid` _asbp_bubble
        (:`Is Valid`
          (bind _result (`self.RemoveDuck` (`/Game/00_Prog/Game/GPE/Bubble/BP_Bubble.capturedActor` _asbp_bubble)))
          (if _result
            _))))
    (:`CastFailed`
      (bind _asbp_main_character (cast `/Game/00_Prog/CCC/BP_MainCharacter` OtherActor))
      (if (< (* (`.SphereRadius` (`KismetSystemLibrary.GetComponentBounds` _enclosurebox)) 0.8) (`KismetMathLibrary.Vector_Distance` (`self.K2_GetActorLocation` _asbp_main_character) (`SceneComponent.K2_GetComponentLocation` _enclosurebox)))
        (bind _holdbubble (`/Game/00_Prog/CCC/BP_Weapon.holdBubble` (`/Game/00_Prog/CCC/BP_MainCharacter.Weapon` _asbp_main_character)))
        (`/Engine/EditorBlueprintResources/StandardMacros.IsValid` _holdbubble
          (:`Is Valid`
            (bind _result_2 (`self.RemoveDuck` (`/Game/00_Prog/Game/GPE/Bubble/BP_Bubble.capturedActor` _holdbubble)))
            (if _result_2
              _)))))))

(event `self.AttackEnclosure`
  (params (_swiper :type "Swiper Object Reference"))
  (bind _stolenduck (`self.IsAttacked`))
  (`/Engine/EditorBlueprintResources/StandardMacros.IsValid` _stolenduck
    (:`Is Valid`
      (`KismetArrayLibrary.Array_RemoveItem` (`Actor.Tags` _stolenduck) "InEnclosure")
      (`KismetArrayLibrary.Array_RemoveItem` (`self.ducksInEnclosure`) _stolenduck)
      (bind _returnvalue (`self.GetComponentByClass` _stolenduck "/Script/OFC.CaughtComponent"))
      (if (`CaughtComponent.IsInBubble` _returnvalue)
        (bind _asbp_bubble (cast `/Game/00_Prog/Game/GPE/Bubble/BP_Bubble` (`CaughtComponent.bubble` _returnvalue)))
        (`/Game/00_Prog/Game/GPE/Bubble/BP_Bubble.Pop` _asbp_bubble)
        (`Swiper.EnclosureGiveDuck` _swiper _stolenduck)))))

(event `self.ReceiveTick`
  (params (DeltaSeconds :type "Float (single-precision)"))
  (`KismetSystemLibrary.PrintString` (`KismetStringLibrary.Concat_StrStr` (`KismetStringLibrary.Conv_IntToString` (`KismetArrayLibrary.Array_Length` (`self.ducksInEnclosure`))) " in enclosure") true true (struct :`R` 0.611063 :`B` 1.0 :`A` 1.0) DeltaSeconds))

(event `self.GetSpawnPoints`
  (params (_aiManager :type "AIManager Object Reference"))
  (`AIManager.GetSpawnPoint` _aiManager (`self.swiperSpawnPoints`)))

(event `self.ForceField4.OnComponentEndOverlap`
  (params (OverlappedComponent :type "PrimitiveComponent Object Reference") (OtherActor :type "Actor Object Reference") (OtherComp :type "PrimitiveComponent Object Reference") (OtherBodyIndex :type Integer)))

(event `self.ForceField1.OnComponentEndOverlap`
  (params (OverlappedComponent :type "PrimitiveComponent Object Reference") (OtherActor :type "Actor Object Reference") (OtherComp :type "PrimitiveComponent Object Reference") (OtherBodyIndex :type Integer))
  (bind _asbp_bubble (cast `/Game/00_Prog/Game/GPE/Bubble/BP_Bubble` OtherActor))
  (bind _asbp_duck (cast `/Game/00_Prog/IA/BP_Duck` (`/Game/00_Prog/Game/GPE/Bubble/BP_Bubble.capturedActor` _asbp_bubble)))
  (if (`self.ActorHasTag` _asbp_duck "InEnclosure")
    (`KismetArrayLibrary.Array_RemoveItem` (`self.ducksInEnclosure`) _asbp_duck)
    (`KismetArrayLibrary.Array_RemoveItem` (`Actor.Tags` _asbp_duck) "InEnclosure")
    (`KismetSystemLibrary.PrintString` "-1 canard de l'enclos ")))

(event `self.ForceField3.OnComponentEndOverlap`
  (params (OverlappedComponent :type "PrimitiveComponent Object Reference") (OtherActor :type "Actor Object Reference") (OtherComp :type "PrimitiveComponent Object Reference") (OtherBodyIndex :type Integer))
  (bind _asbp_bubble (cast `/Game/00_Prog/Game/GPE/Bubble/BP_Bubble` OtherActor))
  (bind _asbp_duck (cast `/Game/00_Prog/IA/BP_Duck` (`/Game/00_Prog/Game/GPE/Bubble/BP_Bubble.capturedActor` _asbp_bubble)))
  (if (`self.ActorHasTag` _asbp_duck "InEnclosure")
    (`KismetArrayLibrary.Array_RemoveItem` (`self.ducksInEnclosure`) _asbp_duck)
    (`KismetArrayLibrary.Array_RemoveItem` (`Actor.Tags` _asbp_duck) "InEnclosure")
    (`KismetSystemLibrary.PrintString` "-1 canard de l'enclos ")))

(event `self.ForceField2.OnComponentEndOverlap`
  (params (OverlappedComponent :type "PrimitiveComponent Object Reference") (OtherActor :type "Actor Object Reference") (OtherComp :type "PrimitiveComponent Object Reference") (OtherBodyIndex :type Integer))
  (bind _asbp_bubble (cast `/Game/00_Prog/Game/GPE/Bubble/BP_Bubble` OtherActor))
  (bind _asbp_duck (cast `/Game/00_Prog/IA/BP_Duck` (`/Game/00_Prog/Game/GPE/Bubble/BP_Bubble.capturedActor` _asbp_bubble)))
  (if (`self.ActorHasTag` _asbp_duck "InEnclosure")
    (`KismetArrayLibrary.Array_RemoveItem` (`self.ducksInEnclosure`) _asbp_duck)
    (`KismetArrayLibrary.Array_RemoveItem` (`Actor.Tags` _asbp_duck) "InEnclosure")
    (`KismetSystemLibrary.PrintString` "-1 canard de l'enclos ")))

(fn `AddDuckFromBubble`
  (params (Actor :type "/Game/00_Prog/Game/GPE/Bubble/BP_Bubble Object Reference"))
  (returns (Duck :type "Duck Object Reference"))
  (bind _capturedactor (`/Game/00_Prog/Game/GPE/Bubble/BP_Bubble.capturedActor` Actor))
  (if (`KismetSystemLibrary.IsValid` Actor)
    (`/Engine/EditorBlueprintResources/StandardMacros.IsValid` _capturedactor
      (:`Is Valid`
        (if (not (`self.ActorHasTag` _capturedactor "InEnclosure"))
          (bind _asbp_duck (cast `/Game/00_Prog/IA/BP_Duck` _capturedactor)
            (:`then`
              (`KismetArrayLibrary.Array_Add` (`self.ducksInEnclosure`) _asbp_duck)
              (`Duck.UpdateEnclosure` _asbp_duck self)
              (`Duck.NotFree` _asbp_duck)
              (`KismetArrayLibrary.Array_Add` (`Actor.Tags` _asbp_duck) "InEnclosure")
              (`/Game/00_Prog/Game/GPE/Bubble/BP_Bubble.Pop` Actor)
              (`self.K2_SetActorLocation` _asbp_duck (`SceneComponent.K2_GetComponentLocation` (`self.DuckTPSceneComponent`)) false true)
              (return _asbp_duck))
            (:`CastFailed`
              _))))
      (:`Is Not Valid`
        _)))
  (return null))

(fn `AddDuckFromPlayer`
  (params (Actor :type "/Game/00_Prog/CCC/BP_MainCharacter Object Reference"))
  (returns (Duck :type "Duck Object Reference"))
  (bind _holdbubble (`/Game/00_Prog/CCC/BP_Weapon.holdBubble` (`/Game/00_Prog/CCC/BP_MainCharacter.Weapon` Actor)))
  (bind _capturedactor (`/Game/00_Prog/Game/GPE/Bubble/BP_Bubble.capturedActor` _holdbubble))
  (`/Engine/EditorBlueprintResources/StandardMacros.IsValid` _holdbubble
    (:`Is Valid`
      (`/Engine/EditorBlueprintResources/StandardMacros.IsValid` _capturedactor
        (:`Is Valid`
          (if (not (`self.ActorHasTag` _capturedactor "InEnclosure"))
            (bind _asduck (cast `Duck` _capturedactor))
            (`KismetArrayLibrary.Array_Add` (`self.ducksInEnclosure`) _asduck)
            (`Duck.UpdateEnclosure` _asduck self)
            (`Duck.NotFree` _asduck)
            (`KismetArrayLibrary.Array_Add` (`Actor.Tags` _asduck) "InEnclosure")
            (return _asduck)))))))

(fn `IsAttacked`
  (returns (stolenDuck :type "Duck Object Reference"))
  (bind _ducksinenclosure (`self.ducksInEnclosure`))
  (if (`KismetArrayLibrary.Array_IsEmpty` _ducksinenclosure)
    (return null)
    (else
      (return (`|GetArrayItem` _ducksinenclosure)))))

(fn `RemoveDuck`
  (params (Object :type "Actor Object Reference"))
  (returns (result :type Boolean))
  (`/Engine/EditorBlueprintResources/StandardMacros.IsValid` Object
    (:`Is Valid`
      (bind _asbp_duck (cast `/Game/00_Prog/IA/BP_Duck` Object)
        (:`then`
          (if (`self.ActorHasTag` _asbp_duck "InEnclosure")
            (`KismetArrayLibrary.Array_RemoveItem` (`self.ducksInEnclosure`) _asbp_duck)
            (bind _returnvalue (`KismetArrayLibrary.Array_RemoveItem` (`Actor.Tags` _asbp_duck) "InEnclosure"))
            (`Duck.UpdateEnclosure` _asbp_duck null)
            (return _returnvalue)
            (else
              (return false))))
        (:`CastFailed`
          (return false))))
    (:`Is Not Valid`
      (return false))))

(fn `UserConstructionScript`)