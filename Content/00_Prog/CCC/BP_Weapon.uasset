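; Player bubble gun, owned by BP_MainCharacter, that shoots bubbles of the current element and vacuums existing ones to hold and throw.
; While sucking, Tick sphere-traces toward the camera aim point and pulls bubbles with distance-scaled force until Detection catches one at the Muzzle.
; Catching a BP_BubbleSwitch changes the element and shrinks it through the Absorb timeline.
; Shots use camera-trace aiming, a cooldown and added forward character velocity.
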(event `self.ReceiveBeginPlay`
  (bind _asbp_main_character (cast `/Game/00_Prog/CCC/BP_MainCharacter` (`self.GetParentActor`)))
  (set `self.Character` _asbp_main_character))

(event `Absorb`
  (bind (_direction _scale) (`Timeline|Absorb_Bubble` :!via `PlayFromStart`)
    (:`Update`
      (`self.SetActorScale3D` (`self.holdBubble`) (`KismetMathLibrary.MakeVector` _scale _scale _scale)))
    (:`Finished`
      (set `self.SwitchingElement?` false)
      (bind _asbp_bubble_switch (cast `/Game/00_Prog/Game/GPE/Bubble/Switcher/BP_BubbleSwitch` (`self.holdBubble`)))
      (`/Game/00_Prog/Game/GPE/Bubble/Switcher/BP_BubbleSwitch.TellSwitcherToRespawnBubble` _asbp_bubble_switch)
      (set `self.holdBubble` null))))

(event `self.ReceiveTick`
  (params (DeltaSeconds :type "Float (single-precision)"))
  (bind _returnvalue (`self.K2_GetActorLocation`))
  (if (`self.Sucking?`)
    ;[1 1 1] Suck
    (bind (_outhits _returnvalue_2) (`KismetSystemLibrary.SphereTraceMultiForObjects` (`self.K2_GetActorLocation`) (`self.GetAimInfo` true) (`self.VacuumRadius`) (`|MakeArray` "ObjectTypeQuery7" :!type "EObjectTypeQuery Enum") false (`|MakeArray` self (`self.GetParentActor`) :!type "Actor Object Reference") "ForOneFrame"))
    (if _returnvalue_2
      (for _array_element _outhits
        (bind _asbp_bubble (cast `/Game/00_Prog/Game/GPE/Bubble/BP_Bubble` (`.HitActor` (`GameplayStatics.BreakHitResult` _array_element))))
        (bind _returnvalue_3 (`self.K2_GetActorLocation` _asbp_bubble))
        (bind _returnvalue_4 (`KismetMathLibrary.Vector_Distance` _returnvalue_3 _returnvalue))
        (`/Game/00_Prog/Game/GPE/Bubble/BP_Bubble.Suck` _asbp_bubble (* (`KismetMathLibrary.GetDirectionUnitVector` _returnvalue_3 _returnvalue) (`KismetMathLibrary.MapRangeClamped` _returnvalue_4 (`self.SuckDist_Min`) (`self.SuckDist_Max`) (`self.SuckSpeed_Max`) (`self.SuckSpeed_Min`)) (`self.SuckSpeed_Modifier`)) (* (`KismetMathLibrary.MapRangeClamped` _returnvalue_4 (`self.SuckDist_Min`) (`self.SuckDist_Max`) (`self.SuckRot_Max`) (`self.SuckRot_Min`)) (`self.SuckSpeed_Modifier`)))))))

(event `Shoot`
  (bind _returnvalue (`KismetMathLibrary.GetForwardVector` (`.LookAtRotation` (`self.GetAimInfo` false))))
  (bind (_returnvalue_location _returnvalue_rotation) (`KismetMathLibrary.BreakTransform` (`SceneComponent.GetSocketTransform` (`self.StaticMesh`) "Muzzle" "RTS_World")))
  ;[1 1 1] Shooting
  (if (not (or (`self.Shooting?`) (`self.Sucking?`) (`self.SwitchingElement?`)))
    (`|ExecutionSequence`
      (:`then_0`
        (set `self.Shooting?` true)
        (bind _returnvalue_2 (`NiagaraFunctionLibrary.SpawnSystemAtLocation` "/Game/04_FX/NS/Player/NS_Gun_Shoot.NS_Gun_Shoot" _returnvalue_location _returnvalue_rotation))
        (`NiagaraComponent.SetVariableMaterial` _returnvalue_2 "Bubble_Mat" (select `/Game/00_Prog/Utils/E_BubbleTypes` (`/Game/00_Prog/Utils/BFL_Bubbles.getBubbleEnumFromClass` (`self.currentBubbleType`)) :`NewEnumerator0` "/Game/04_FX/Ressources/Mat/MIFX_Bubble.MIFX_Bubble" :`NewEnumerator1` "/Game/04_FX/Ressources/Mat/MIFX_ChewingGum_Bubble.MIFX_ChewingGum_Bubble" :`NewEnumerator2` "/Game/04_FX/Ressources/Mat/MIFX_Oil_Bubble.MIFX_Oil_Bubble" :`NewEnumerator3` "/Game/04_FX/Ressources/Mat/MIFX_mercury_Bubble.MIFX_mercury_Bubble" :`NewEnumerator4` "/Game/04_FX/Ressources/Mat/MIFX_Nuggets.MIFX_Nuggets" :!type "MaterialInterface Object Reference"))
        (`KismetSystemLibrary.Delay` (* (`self.ShootCooldown`) (`self.ShootCooldownModifier`)))
        (set `self.Shooting?` false))
      (:`then_1`
        (if (`self.HoldingBubble?`)
          (set `self.HoldingBubble?` false)
          (`self.K2_DetachFromActor` (`self.holdBubble`) "KeepWorld" "KeepWorld" "KeepWorld")
          (`/Game/00_Prog/Game/GPE/Bubble/BP_Bubble.Throw` (`self.holdBubble`) (`self.AddCharVelocity` (* _returnvalue (`self.ShootForce`) (`self.BubbleLaunchSpeedModifier`) (`KismetMathLibrary.SelectFloat` (`self.ChewingGum_ShootMod`) 1.0 (== (`GameplayStatics.GetObjectClass` (`self.holdBubble`)) "/Game/00_Prog/Game/GPE/Bubble/BP_ChewingGumBubble.BP_ChewingGumBubble_C"))) _returnvalue))
          (set `self.holdBubble` null)
          (else
            (bind _returnvalue_3 (`|SpawnActorFromClass` (`self.currentBubbleType`) (`KismetMathLibrary.MakeTransform` (`self.K2_GetActorLocation`) (`.LookAtRotation` (`self.GetAimInfo` false))) "AlwaysSpawn" "MultiplyWithRoot" null null))
            (bind _returnvalue_4 (`self.GetActorForwardVector` _returnvalue_3))
            (`/Game/00_Prog/Game/GPE/Bubble/BP_Bubble.Shoot` _returnvalue_3 (`self.AddCharVelocity` (* _returnvalue_4 (`self.ShootForce`) (`self.BubbleLaunchSpeedModifier`) (`KismetMathLibrary.SelectFloat` (`self.ChewingGum_ShootMod`) 1.0 (== (`self.currentBubbleType`) "/Game/00_Prog/Game/GPE/Bubble/BP_ChewingGumBubble.BP_ChewingGumBubble_C"))) _returnvalue_4))))))))

(event `StartSuck`
  ;[1 1 1] Sucking
  (if (not (or (`self.Sucking?`) (`self.HoldingBubble?`) (`self.SwitchingElement?`)))
    (set `self.Sucking?` true)
    (`self.SetActorTickEnabled` true)
    (for _array_element (`PrimitiveComponent.GetOverlappingActors` (`self.Detection`) "/Game/00_Prog/Game/GPE/Bubble/BP_Bubble.BP_Bubble_C")
      (bind _caughtabubble_ (`self.CatchBubble` _array_element))
      (if _caughtabubble_
        (break)))
    (if (not (`KismetSystemLibrary.IsValid` (`self.holdBubble`)))
      (`|ExecutionSequence`
        (:`then_0`
          (bind _sound_vacuum (`self.Sound_Vacuum`)
            (:`then`
              (`AudioComponent.Play` _sound_vacuum 0.0))
            (:`else`
              (bind _returnvalue (`GameplayStatics.SpawnSound2D` "/Game/05_Audio/SFX/Metasounds/Player_Character/Char_Vacuum_Bubbles/MSS_Char_Vaccum_Bubbles_v2.MSS_Char_Vaccum_Bubbles_v2" 0.5 1.0 0.0 null false false))
              (set `self.Sound_Vacuum` _returnvalue))))
        (:`then_1`
          (`self.VacuumVFX`
            (:`then`)
            (:`else`
              (bind _returnvalue_2 (`NiagaraFunctionLibrary.SpawnSystemAttached` "/Game/04_FX/NS/Player/NS_Aspirate.NS_Aspirate" (`self.StaticMesh`) "Muzzle" (0.0 0.0 0.0) (struct) "KeepRelativeOffset"))
              (set `self.VacuumVFX` _returnvalue_2))))))))

(event `StopSuck`
  ;[1 1 1] Sucking
  (if (not (or (`self.HoldingBubble?`) (`self.SwitchingElement?`)))
    (set `self.Sucking?` false)
    (`self.SetActorTickEnabled` false)
    (`|ExecutionSequence`
      (:`then_0`
        (bind _sound_vacuum (`self.Sound_Vacuum`)
          (:`then`
            (`AudioComponent.FadeOut` _sound_vacuum 0.5 0.0 "Logarithmic"))
          (:`else`)))
      (:`then_1`
        (bind _vacuumvfx (`self.VacuumVFX`)
          (:`then`
            (`ActorComponent.K2_DestroyComponent` _vacuumvfx))
          (:`else`))))))

(event `self.Detection.OnComponentBeginOverlap`
  (params (OverlappedComponent :type "PrimitiveComponent Object Reference") (OtherActor :type "Actor Object Reference") (OtherComp :type "PrimitiveComponent Object Reference") (OtherBodyIndex :type Integer) (bFromSweep :type Boolean) (SweepResult :type "HitResult Structure (by ref)"))
  (`self.CatchBubble` OtherActor))

(event `SwitchElement`
  (params (BubbleType :type "/Game/00_Prog/Game/GPE/Bubble/BP_Bubble Class Reference"))
  (set `self.currentBubbleType` BubbleType)
  (set `self.SwitchingElement?` true)
  (`self.Absorb`))

(fn `AddCharVelocity`
  (params (BaseForce :type "Vector Structure") (Direction :type "Vector Structure"))
  (returns (ReturnValue :type "Vector Structure"))
  (bind _velocity (`MovementComponent.Velocity` (`Character.CharacterMovement` (`self.Character`))))
  (return (+ BaseForce (* (`KismetMathLibrary.FMax` (`KismetMathLibrary.Dot_VectorVector` Direction (`KismetMathLibrary.Normal` _velocity))) _velocity))))

(fn `CatchBubble`
  (params (Actor :type "Actor Object Reference"))
  (returns (`CaughtABubble?` :type Boolean))
  (if (and (not (`self.HoldingBubble?`)) (`self.Sucking?`))
    (bind _asbp_bubble (cast `/Game/00_Prog/Game/GPE/Bubble/BP_Bubble` Actor)
      (:`then`
        (if (not (`/Game/00_Prog/Game/GPE/Bubble/BP_Bubble.NewBubble?` _asbp_bubble))
          (`self.StopSuck`)
          (`|ExecutionSequence`
            (:`then_0`
              (bind _output_get (set `self.holdBubble` _asbp_bubble))
              (`/Game/00_Prog/Game/GPE/Bubble/BP_Bubble.CaughtByWeapon` _output_get)
              (`self.K2_AttachToComponent` _asbp_bubble (`self.StaticMesh`) "Muzzle" "SnapToTarget" "SnapToTarget" "KeepWorld" true)
              (bind _asbp_bubble_switch (cast `/Game/00_Prog/Game/GPE/Bubble/Switcher/BP_BubbleSwitch` _asbp_bubble)
                (:`then`
                  (set `self.holdBubble` _asbp_bubble_switch)
                  (`self.SwitchElement` (`/Game/00_Prog/Game/GPE/Bubble/Switcher/BP_BubbleSwitch.bubbleSwitchType` _asbp_bubble_switch)))
                (:`CastFailed`
                  (set `self.HoldingBubble?` true)
                  (`GameplayStatics.PlaySound2D` "/Game/05_Audio/SFX/Metasounds/Player_Character/Char_SuckIn_Bubble/MSS_Char_SuckIn_Bubble.MSS_Char_SuckIn_Bubble" 0.75 1.0 0.0 null null)
                  (message `/Game/00_Prog/Utils/BI_Bubble.OnHeld` (`self.holdBubble`)))))
            (:`then_1`
              (return true)))
          (else
            (return false))))
      (:`CastFailed`
        (return false)))
    (else
      (return false))))

(fn `GetAimInfo`
  (params (`Vacuum?` :type Boolean))
  (returns (LookAtLocation :type "Vector Structure") (LookAtRotation :type "Rotator Structure"))
  (locals (EndPoint :type "Vector Structure"))
  (bind _endpoint (`local.EndPoint`))
  (bind _camera (`/Game/00_Prog/CCC/BP_MainCharacter.Camera` (`self.Character`)))
  (bind _camera_2 (`/Game/00_Prog/CCC/BP_MainCharacter.Camera` (`self.Character`)))
  (bind _returnvalue (`SceneComponent.K2_GetComponentLocation` _camera_2))
  (`|ExecutionSequence`
    (:`then_0`
      (bind _output_get (set `local.EndPoint` (+ _returnvalue (* (`SceneComponent.GetForwardVector` _camera_2) (`KismetMathLibrary.SelectFloat` (`self.VacuumTraceLength`) (`self.AimMinTraceLength`) `Vacuum?`)))))
      (bind (_outhit _returnvalue_2) (`KismetSystemLibrary.LineTraceSingle` _returnvalue _output_get "TraceTypeQuery1" false (`|MakeArray` (`self.Character`) self :!type "Actor Object Reference") "ForDuration" true (struct :`R` 1.0 :`A` 1.0) (struct :`G` 1.0 :`A` 1.0) 0.2))
      (if _returnvalue_2
        (set `local.EndPoint` (`.ImpactPoint` (`GameplayStatics.BreakHitResult` _outhit)))
        (elif (not `Vacuum?`)
          (set `local.EndPoint` (+ (`SceneComponent.K2_GetComponentLocation` _camera) (* (`SceneComponent.GetForwardVector` _camera) (`self.AimMaxTraceLength`)))))))
    (:`then_1`
      (return _endpoint (`KismetMathLibrary.FindLookAtRotation` (`self.K2_GetActorLocation`) _endpoint)))))

(fn `UserConstructionScript`)