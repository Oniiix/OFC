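; Player character Blueprint that handles movement, a clamped spring-arm camera, jumping, weapon use and pausing through Enhanced Input.
; Movement follows the spring arm's orientation, and shoot and suck inputs are forwarded to a BP_Weapon cached from a child actor.
; Pausing swaps player and menu mapping contexts, pauses the game and shows the pause widget.
; Unpausing sets cursor and input mode from the HUD's current state.
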(event `self.ReceiveBeginPlay`
  (`|ExecutionSequence`
    (:`then_0`
      (`EnhancedInputSubsystemInterface.AddMappingContext` (pcsubsystem `EnhancedInputLocalPlayerSubsystem` (`GameplayStatics.GetPlayerController` 0)) "/Game/00_Prog/CCC/Inputs/Context/IMC_Player.IMC_Player" 0 (struct)))
    (:`then_1`
      (bind _asbp_weapon (cast `/Game/00_Prog/CCC/BP_Weapon` (`ChildActorComponent.ChildActor` (`self.Weapon_ChildActor`)))
        (:`then`
          (set `self.Weapon` _asbp_weapon))
        (:`CastFailed`
          (`KismetSystemLibrary.PrintString` "Failed Cast Bp_Weapon"))))))

(event `EnhancedInput|/Game/00_Prog/CCC/Inputs/Actions/Move`
  (params (ActionValue :type "Vector2D Structure") (ElapsedSeconds :type "Float (double-precision)") (TriggeredSeconds :type "Float (double-precision)") (InputAction :type "InputAction Object Reference" :default "/Game/00_Prog/CCC/Inputs/Actions/Move.Move"))
  (bind (_x _y) (`KismetMathLibrary.BreakVector2D` ActionValue))
  (bind _springarm (`self.SpringArm`))
  (bind (_returnvalue_roll _returnvalue_pitch _returnvalue_yaw) (`KismetMathLibrary.BreakRotator` (`SceneComponent.K2_GetComponentRotation` _springarm)))
  (bind (_returnvalue_roll_2 _returnvalue_pitch_2 _returnvalue_yaw_2) (`KismetMathLibrary.BreakRotator` (`SceneComponent.K2_GetComponentRotation` _springarm)))
  ;[1 1 1] INPUTS
  (:`Triggered`
    (`self.AddMovementInput` (`KismetMathLibrary.Normal` (+ (* (`KismetMathLibrary.GetForwardVector` (`KismetMathLibrary.MakeRotator` 0.0 0.0 _returnvalue_yaw_2)) _x) (* _y (`KismetMathLibrary.GetRightVector` (`KismetMathLibrary.MakeRotator` 0.0 _returnvalue_pitch _returnvalue_yaw))))))))

(event `EnhancedInput|/Game/00_Prog/CCC/Inputs/Actions/Rotate`
  (params (ActionValue :type "Float (double-precision)") (ElapsedSeconds :type "Float (double-precision)") (TriggeredSeconds :type "Float (double-precision)") (InputAction :type "InputAction Object Reference" :default "/Game/00_Prog/CCC/Inputs/Actions/Rotate.Rotate"))
  ;[1 1 1] INPUTS
  ;;[1 1 1] Camera
  (:`Triggered`
    (`SceneComponent.K2_AddRelativeRotation` (`self.SpringArm`) (`KismetMathLibrary.MakeRotator` 0.0 0.0 ActionValue) false false)))

(event `EnhancedInput|/Game/00_Prog/CCC/Inputs/Actions/Pitch`
  (params (ActionValue :type "Float (double-precision)") (ElapsedSeconds :type "Float (double-precision)") (TriggeredSeconds :type "Float (double-precision)") (InputAction :type "InputAction Object Reference" :default "/Game/00_Prog/CCC/Inputs/Actions/Pitch.Pitch"))
  ;[1 1 1] INPUTS
  ;;[1 1 1] Camera
  (:`Triggered`
    (`self.SetupPitch` ActionValue)))

(event `EnhancedInput|/Game/00_Prog/CCC/Inputs/Actions/Jump`
  (params (ActionValue :type Boolean) (ElapsedSeconds :type "Float (double-precision)") (TriggeredSeconds :type "Float (double-precision)") (InputAction :type "InputAction Object Reference" :default "/Game/00_Prog/CCC/Inputs/Actions/Jump.Jump"))
  ;[1 1 1] INPUTS
  (:`Started`
    (`self.Jump`)
    ;;[1 1 1] Jump Launch Sound
    (if (`CharacterMovementComponent.IsWalking` (`self.CharacterMovement`))
      (`GameplayStatics.PlaySound2D` "/Game/05_Audio/SFX/Metasounds/Player_Character/Jump_Launch/MSS_Jump_Launch.MSS_Jump_Launch" 1.0 1.0 0.0 null null false))))

(event `EnhancedInput|/Game/00_Prog/CCC/Inputs/Actions/Escape`
  (params (ActionValue :type Boolean) (ElapsedSeconds :type "Float (double-precision)") (TriggeredSeconds :type "Float (double-precision)") (InputAction :type "InputAction Object Reference" :default "/Game/00_Prog/CCC/Inputs/Actions/Escape.Escape"))
  ;[1 1 1] INPUTS
  (:`Started`
    (`self.SetPauseState` (not (`self.inMenu`)))))

(event `EnhancedInput|/Game/00_Prog/CCC/Inputs/Actions/Shoot`
  (params (ActionValue :type Boolean) (ElapsedSeconds :type "Float (double-precision)") (TriggeredSeconds :type "Float (double-precision)") (InputAction :type "InputAction Object Reference" :default "/Game/00_Prog/CCC/Inputs/Actions/Shoot.Shoot"))
  ;[1 1 1] INPUTS
  (:`Triggered`
    (`/Game/00_Prog/CCC/BP_Weapon.Shoot` (`self.Weapon`))))

(event `EnhancedInput|/Game/00_Prog/CCC/Inputs/Actions/Suck`
  (params (ActionValue :type Boolean) (ElapsedSeconds :type "Float (double-precision)") (TriggeredSeconds :type "Float (double-precision)") (InputAction :type "InputAction Object Reference" :default "/Game/00_Prog/CCC/Inputs/Actions/Suck.Suck"))
  (bind _weapon (`self.Weapon`))
  ;[1 1 1] INPUTS
  (:`Triggered`
    (`/Game/00_Prog/CCC/BP_Weapon.StartSuck` _weapon))
  (:`Completed`
    (`/Game/00_Prog/CCC/BP_Weapon.StopSuck` _weapon)))

(fn `ChangeHUDState`
  (params (newState :type "UEnumUI Enum" :default "MainMenu"))
  (bind _asbp_base_hud (cast `/Game/00_Prog/UI/HUD/Bp_BaseHUD` (`PlayerController.GetHUD` (`GameplayStatics.GetPlayerController` 0))))
  (`/Game/00_Prog/UI/HUD/Bp_BaseHUD.SetState` _asbp_base_hud newState))

(fn `SetPauseState`
  (params (State :type Boolean))
  (bind _returnvalue (`GameplayStatics.GetPlayerController` 0))
  (bind _inmenu (`self.inMenu`))
  (set `self.inMenu` State)
  (`self.UpdateMappingContext` (select `bool` _inmenu :`false` "/Game/00_Prog/CCC/Inputs/Context/IMC_Menu.IMC_Menu" :`true` "/Game/00_Prog/CCC/Inputs/Context/IMC_Player.IMC_Player" :!type "InputMappingContext Object Reference") (select `bool` _inmenu :`false` "/Game/00_Prog/CCC/Inputs/Context/IMC_Player.IMC_Player" :`true` "/Game/00_Prog/CCC/Inputs/Context/IMC_Menu.IMC_Menu" :!type "InputMappingContext Object Reference"))
  (`GameplayStatics.SetGamePaused` (`self.inMenu`))
  (if (`self.inMenu`)
    (bind _returnvalue_2 (`|CreateWidget` "/Game/00_Prog/UI/MainMenu/Bp_PauseMenu.Bp_PauseMenu_C" (`GameplayStatics.GetPlayerController` 0)))
    (bind _output_get (set `self.PauseWidget` _returnvalue_2))
    (`UserWidget.AddToViewport` _output_get 0)
    (set `PlayerController.bShowMouseCursor` true (`GameplayStatics.GetPlayerController` 0))
    (`WidgetBlueprintLibrary.SetInputMode_GameAndUIEx` (`GameplayStatics.GetPlayerController` 0) (`self.PauseWidget`) "LockInFullscreen" false)
    (else
      (`Widget.RemoveFromParent` (`self.PauseWidget`))
      (set `self.PauseWidget` null)
      (bind _asbp_base_hud (cast `/Game/00_Prog/UI/HUD/Bp_BaseHUD` (`PlayerController.GetHUD` (`GameplayStatics.GetPlayerController` 0))))
      (if (`|EnumEquality` (`/Game/00_Prog/UI/HUD/Bp_BaseHUD.CurrentState` _asbp_base_hud) "Game")
        (set `PlayerController.bShowMouseCursor` false _returnvalue)
        (`WidgetBlueprintLibrary.SetInputMode_GameOnly` _returnvalue)
        (else
          (`WidgetBlueprintLibrary.SetInputMode_GameAndUIEx` (`GameplayStatics.GetPlayerController` 0) (`/Game/00_Prog/UI/HUD/Bp_BaseHUD.LastWidget` _asbp_base_hud) "LockInFullscreen" false))))))

(fn `SetupPitch`
  (params (B :type "Float (double-precision)"))
  (bind __newpitchx (`self._newPitchX`))
  (`self.UpdatePitchX` B)
  (`self.UpdatePitchY` B)
  (if (<= __newpitchx -80.0)
    (`self.SetupPitchLimit` -80.0)
    (elif (>= __newpitchx 80.0)
      (`self.SetupPitchLimit` 80.0)
      (else
        (`SceneComponent.K2_AddLocalRotation` (`self.SpringArm`) (* (`KismetMathLibrary.MakeRotator` 0.0 1.0) B) false false)))))

(fn `SetupPitchLimit`
  (params (pitch :type "Float (double-precision)"))
  (bind _springarm (`self.SpringArm`))
  (`SceneComponent.K2_SetRelativeRotation` _springarm (`KismetMathLibrary.MakeRotator` (.roll (`SceneComponent.RelativeRotation` _springarm)) pitch (.yaw (`SceneComponent.RelativeRotation` _springarm))) false false))

(fn `UpdateMappingContext`
  (params (contextToRemove :type "InputMappingContext Object Reference") (contextToAdd :type "InputMappingContext Object Reference"))
  (bind _returnvalue (pcsubsystem `EnhancedInputLocalPlayerSubsystem` (`GameplayStatics.GetPlayerController` 0)))
  (`EnhancedInputSubsystemInterface.RemoveMappingContext` _returnvalue contextToRemove (struct))
  (`EnhancedInputSubsystemInterface.AddMappingContext` _returnvalue contextToAdd 0 (struct)))

(fn `UpdatePause`
  (params (contextToRemove :type "InputMappingContext Object Reference") (contextToAdd :type "InputMappingContext Object Reference") (newState :type "UEnumUI Enum" :default "MainMenu"))
  (`self.UpdateMappingContext` contextToRemove contextToAdd)
  (`self.ChangeHUDState` newState))

(fn `UpdatePitchX`
  (params (B :type "Float (double-precision)"))
  (set `self._newPitchX` (+ (.pitch (`SceneComponent.RelativeRotation` (`self.SpringArm`))) B))
  (return))

(fn `UpdatePitchY`
  (params (B :type "Float (double-precision)"))
  (set `self._newPitchY` (- (.pitch (`SceneComponent.RelativeRotation` (`self.SpringArm`))) B)))

(fn `UserConstructionScript`)