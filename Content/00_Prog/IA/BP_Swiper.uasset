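; BP_Swiper is an AI actor that tracks whether it is bubbled or has caught a duck.
; On BeginPlay it binds to its bubbled, pop-bubbled and catch-duck dispatchers, then plays a spawn sound at its location.
; The handlers only set the Bubbled and Catch flags, with being bubbled also clearing the catch.
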(event `self.ReceiveBeginPlay`
  (add `self.onPopBubbled` (delegate `onPopBubbled_Event`))
  (add `self.onCatchDuck` (delegate `onCatchDuck_Event`))
  (add `self.onBubbled` (delegate `onBubbled_Event`))
  (`GameplayStatics.PlaySoundAtLocation` (`self.Spawn_SFX`) (`self.K2_GetActorLocation`) (struct) (`self.Spawn_Volume`) 1.0 0.0 null null null null))

(event `onPopBubbled_Event`
  (set `self.Bubbled?` false))

(event `onCatchDuck_Event`
  (set `self.Catch?` true))

(event `onBubbled_Event`
  (set `self.Bubbled?` true)
  (set `self.Catch?` false))

(fn `UserConstructionScript`)