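; BP_Duck is a duck creature that can be chased by a swiper, kidnapped, bubbled, held, thrown and killed.
; On BeginPlay it binds to its state dispatchers, whose handlers, along with held and thrown events, maintain boolean state flags.
; These events also drive feedback: feathers and a burst sound on death, a panic sound when bubbled, and an attached panic loop when kidnapped or held that fades out when thrown.
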(event `self.ReceiveBeginPlay`
  (add `self.onDead` (delegate `onDead_Event`))
  (add `self.onDetectSwiper` (delegate `onDetectSwiper_Event`))
  (add `self.onBubbled` (delegate `onBubbled_Event`))
  (add `self.onKidnapped` (delegate `onKidnapped_Event`))
  (add `self.onStop` (delegate `onStop_Event`))
  (add `self.onWalking` (delegate `onWalking_Event`))
  (add `self.onPopBubbled` (delegate `onPopBubbled_Event`)))

(event `onDead_Event` :!signature `self.onDead`
  (params (_this :type "Duck Object Reference"))
  (`NiagaraFunctionLibrary.SpawnSystemAtLocation` "/Game/04_FX/NS/Ducks/NS_Feathers.NS_Feathers" (`self.K2_GetActorLocation` _this))
  (`GameplayStatics.PlaySoundAtLocation` "/Game/05_Audio/SFX/Metasounds/Bubbles/Bubble_Burst/MSS_Bubble_Burst_Light.MSS_Bubble_Burst_Light" (`self.K2_GetActorLocation`) (struct) 0.75 1.0 0.0 null null null null))

(event `onDetectSwiper_Event`
  (set `self.Chased?` true))

(event `onBubbled_Event`
  (set `self.Bubbled?` true)
  (set `self.Grabbed?` false)
  (`GameplayStatics.PlaySoundAtLocation` "/Game/05_Audio/SFX/Metasounds/Duck/Duck_Run_Panik/MSS_A_D_Run_Panik_v2.MSS_A_D_Run_Panik_v2" (`self.K2_GetActorLocation`) (struct) 1.0 1.0 0.0 null null null null))

(event `onPopBubbled_Event`
  (set `self.Bubbled?` false)
  (set `self.Held?` false)
  (set `self.Thrown?` false))

(event `onKidnapped_Event`
  (set `self.Grabbed?` true)
  (bind _panickedsound (`self.PanickedSound`)
    (:`then`
      (`AudioComponent.Play` _panickedsound 0.0))
    (:`else`
      (bind _returnvalue (`GameplayStatics.SpawnSoundAttached` "/Game/05_Audio/SFX/Metasounds/Duck/Bubbled_Panik/MSS_Bubbled_Panik.MSS_Bubbled_Panik" (`self.Mesh`) "mouth" (0.0 0.0 0.0) (struct) "KeepRelativeOffset" true 0.75 1.0 0.0 null null))
      (set `self.PanickedSound` _returnvalue))))

(event `onStop_Event`)

(event `onWalking_Event`
  (set `self.Chased?` false)
  (set `self.Grabbed?` false))

(event `/Game/00_Prog/Utils/BI_Bubble.OnHeld`
  (set `self.Held?` true)
  (bind _returnvalue (`GameplayStatics.SpawnSoundAttached` "/Game/05_Audio/SFX/Metasounds/Duck/Bubbled_Panik/MSS_Bubbled_Panik.MSS_Bubbled_Panik" (`self.Mesh`) "mouth" (0.0 0.0 0.0) (struct) "KeepRelativeOffset" true 0.75 1.0 0.0 null null))
  (set `self.PanickedSound` _returnvalue))

(event `/Game/00_Prog/Utils/BI_Bubble.OnThrown`
  (set `self.Thrown?` true)
  (set `self.Held?` false)
  (bind _panickedsound (`self.PanickedSound`)
    (:`then`
      (`AudioComponent.FadeOut` _panickedsound 0.2 0.0 "Linear"))
    (:`else`)))

(event `self.CapsuleComponent.OnComponentEndOverlap`
  (params (OverlappedComponent :type "PrimitiveComponent Object Reference") (OtherActor :type "Actor Object Reference") (OtherComp :type "PrimitiveComponent Object Reference") (OtherBodyIndex :type Integer)))

(fn `UserConstructionScript`)