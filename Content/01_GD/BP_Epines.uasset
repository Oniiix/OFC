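; BP_Epines is a thorns prop that marks its static mesh with the piercing tag at BeginPlay.
; The construction script adds a random yaw to the mesh for visual variety.
; SnapToGround traces a short distance down from the Sphere against one object type, then teleports the actor to the hit, aligned to the surface normal.
; Nothing in this graph calls SnapToGround.
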(event `self.ReceiveBeginPlay`
  (`KismetArrayLibrary.Array_Add` (`ActorComponent.ComponentTags` (`self.StaticMesh`)) (`/Game/00_Prog/Utils/BFL_Piercing.GetPiercingTagName`)))

(fn `SnapToGround`
  (bind _returnvalue (`SceneComponent.K2_GetComponentLocation` (`self.Sphere`)))
  (bind (_outhit _returnvalue_2) (`KismetSystemLibrary.LineTraceSingleForObjects` _returnvalue (+ _returnvalue (0.0 0.0 -100.0)) (`|MakeArray` "ObjectTypeQuery10" :!type "EObjectTypeQuery Enum")))
  (if _returnvalue_2
    (bind (_bblockinghit _binitialoverlap _time _distance _location _impactpoint _normal) (`GameplayStatics.BreakHitResult` _outhit))
    (`self.K2_SetActorLocationAndRotation` _location (`KismetMathLibrary.MakeRotFromZX` _normal (`self.GetActorForwardVector`)) false true)))

(fn `UserConstructionScript`
  (`SceneComponent.K2_AddRelativeRotation` (`self.StaticMesh`) (`KismetMathLibrary.MakeRotator` 0.0 0.0 (`KismetMathLibrary.RandomFloatInRange` 0.0 360.0)) false false))